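; Fighters shop actor that registers itself with the training ground game mode on BeginPlay and generates a random roster of fighters.
; GenerateFighters derives a level range from the average level of the player's fighters.
; Each new fighter draws a name from the Names table, randomized stats within that range, and required XP from ExpList.
; All get the same test sword and a -2 player-array index.
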(event Custom|GenerateFighters
  (Utilities|Array|Clear (Variables|Default|GetFighters))
  (bind _asplayer_controller (Utilities|Casting|CastToPlayerController (Game|GetPlayerController 0)))
  (Variables|Default|SetaverageLVL 0)
  (for _array_element (Variables|/Game/Blueprints/PlayerController.PlayerController_C|GetPlayerFighterList _asplayer_controller)
    (Variables|Default|SetaverageLVL (+ (Variables|Default|GetaverageLVL) (.Level (Utilities|Struct|BreakStruct_Fighter _array_element)))))
  (Variables|Default|SetaverageLVL (/ (Variables|Default|GetaverageLVL) (Utilities|Array|Length (Variables|/Game/Blueprints/PlayerController.PlayerController_C|GetPlayerFighterList _asplayer_controller))))
  (if (> (Variables|Default|GetaverageLVL) 2)
    (Variables|Default|SetminLVL (- (Variables|Default|GetaverageLVL) 1))
    (elif (== (Variables|Default|GetaverageLVL) 0)
      (Variables|Default|SetminLVL 1)
      (else
        (Variables|Default|SetminLVL (Variables|Default|GetaverageLVL)))))
  (Variables|Default|SetmaxLVL (+ (Variables|Default|GetaverageLVL) (Math|Random|RandomIntegerinRange 1 2)))
  (for _index (range 0 (- (Variables|Default|GetNumberOfFighters) 1))
    (bind _outrownames (DataTable|GetDataTableRowNames "/Game/Blueprints/DataTables/Names.Names"))
    (bind _returnvalue (Utilities|GetDataTableRow "/Game/Blueprints/DataTables/Names.Names" (Utilities|Array|Get(acopy) _outrownames (Math|Random|RandomIntegerinRange 0 (- (Utilities|Array|Length _outrownames) 1))))
      (:then
        (Variables|Default|SetLVL (Math|Random|RandomIntegerinRange (Variables|Default|GetminLVL) (Variables|Default|GetmaxLVL)))
        (bind _returnvalue_2 (Utilities|GetDataTableRow "/Game/Blueprints/DataTables/ExpList.ExpList" (Utilities|String|StringToName (Utilities|String|ToString(Integer) (- (Variables|Default|GetLVL) 1))))
          (:then
            (Utilities|Array|Add (Variables|Default|GetFighters) (Utilities|Struct|MakeStruct_Fighter (Utilities|Struct|BreakFigthersNames_Struct _returnvalue) (Variables|Default|GetLVL) (Math|Random|RandomIntegerinRange 1 (Variables|Default|GetLVL)) (- (Variables|Default|GetLVL) (Math|Random|RandomIntegerinRange 1 (Variables|Default|GetLVL))) 0 0.0 (Math|Conversions|ToFloat(Integer) (Math|Float|Round (.EXP (Utilities|Struct|BreakLvlList_Struct _returnvalue_2)))) (Utilities|Struct|MakeStruct_Sword "/Game/Meshes/SkeletalMeshes/Sword_Test_1/Sword_Test_1_SM.Sword_Test_1_SM" 5e+02 2e+01) -2))))))))

(event EventBeginPlay
  (bind _astraining_ground_game_mode (Utilities|Casting|CastToTrainingGroundGameMode (Game|GetGameMode)))
  (Variables|/Game/Blueprints/TrainingGroundGameMode.TrainingGroundGameMode_C|SetFightersShop _astraining_ground_game_mode self))

(event Collision|EventActorBeginOverlap
  (params (OtherActor :type Actor%20Object%20Reference)))

(event EventTick
  (params (DeltaSeconds :type Float%20%28single-precision%29)))

(fn ConstructionScript)