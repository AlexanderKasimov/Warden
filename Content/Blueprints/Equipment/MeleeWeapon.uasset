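; Melee weapon that detects hits along its front and back cutting edges and reports them to damageable actors.
; Every tick it derives swing speed from the model's world-space movement over delta time, then traces both edges.
; Each edge samples points along a spline and fires short, debug-drawn Visibility line traces along the model's forward or reversed forward vector.
; Hit actors implementing IDamagable receive the hit, speed and weapon weight.
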(event EventBeginPlay)

(event Collision|EventActorBeginOverlap
  (params (OtherActor :type Actor%20Object%20Reference)))

(event EventTick
  (params (DeltaSeconds :type Float%20%28single-precision%29))
  (Utilities|FlowControl|Sequence
    (:then_0
      (Variables|Default|SetSpeed (CallFunction|GetSpeed (Transformation|GetWorldLocation (Variables|Default|GetModel)) (Variables|Default|GetLastLocation)))
      (Variables|Default|SetLastLocation (Transformation|GetWorldLocation (Variables|Default|GetModel))))
    (:then_1
      (CallFunction|TraceEdge 1e+01 2e+01 "NewEnumerator0")
      (CallFunction|TraceEdge 1e+01 2e+01 "NewEnumerator1"))))

(fn ConstructionScript
  (|CallParentFunction))

(fn GetSpeed
  (params (CurLocation :type Vector) (LastLocation :type Vector))
  (return (/ (Math|Vector|VectorLength (- CurLocation LastLocation)) (Utilities|Time|GetWorldDeltaSeconds))))

(fn TraceEdge
  (params (Parts :type Float%20%28single-precision%29) (TraceLength :type Float%20%28single-precision%29) (Side :type Enum_Sides%20Enum :default "NewEnumerator0"))
  (LocalVariables|SetLocalParts Parts)
  (LocalVariables|SetLocalTraceLength TraceLength)
  (Utilities|FlowControl|Sequence
    (:then_0
      (switch Utilities|FlowControl|Switch|SwitchonEnum_Sides Side
        (:NewEnumerator0
          (LocalVariables|SetSpline (Variables|Default|GetFrontCuttingEdgeSpline))
          (LocalVariables|SetLocalDirectionVector (Math|Vector|GetForwardVector (Variables|Default|GetModel))))
        (:NewEnumerator1
          (LocalVariables|SetSpline (Variables|Default|GetBackCuttingEdgeSpline))
          (LocalVariables|SetLocalDirectionVector (* (Math|Vector|GetForwardVector (Variables|Default|GetModel)) -1.0)))))
    (:then_1
      (bind _output_get (LocalVariables|SetIntervalLength (/ (Spline|GetSplineLength (LocalVariables|GetSpline)) (LocalVariables|GetLocalParts))))
      (for _index (range 0 (Math|Float|Truncate _output_get))
        (LocalVariables|SetStartPoint (Spline|GetLocationatDistanceAlongSpline (LocalVariables|GetSpline) (LocalVariables|GetPathLength) "World"))
        (LocalVariables|SetPathLength (+ (LocalVariables|GetPathLength) (LocalVariables|GetIntervalLength)))
        (bind (_outhit _returnvalue) (Collision|LineTraceByChannel (LocalVariables|GetStartPoint) (+ (LocalVariables|GetStartPoint) (* (LocalVariables|GetLocalDirectionVector) (LocalVariables|GetLocalTraceLength))) "TraceTypeQuery1" false 0 "ForDuration"))
        (bind _output_get_2 (LocalVariables|SetLocalHitInfo _outhit))
        (if _returnvalue
          (if (Utilities|DoesObjectImplementInterface (.HitActor (Collision|BreakHitResult _output_get_2)) "/Game/Blueprints/iDamagable.iDamagable_C")
            (CallFunction|HitDamagable (LocalVariables|GetLocalHitInfo))))))))

(fn HitDamagable
  (params (HitInfo :type Hit%20Result%20Structure))
  (LocalVariables|SetLocalHitResult HitInfo)
  (Class|IDamagable|RecieveDamage(Message) (.HitActor (Collision|BreakHitResult HitInfo)) (LocalVariables|GetLocalHitResult) 0.0 (Variables|Default|GetSpeed) (Variables|Default|GetWeight)))