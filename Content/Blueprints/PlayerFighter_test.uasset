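; Test player fighter with axis movement, Leap Motion hand tracking, sword combat, health and XP intake.
; The right hand positions a sphere, while a child-actor sword, socketed at construction, turns each Tick toward the last living Fighter found.
; FighterInfo stats set HP and damage, which a sphere-trace attack applies once per enemy via IDamagable, also pushing physics props.
; Incoming hits spawn blood effects, and lethal ones break a bone constraint and ragdoll the body.
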(event Custom|ExpRecieved
  (params (Recieved%20XP :type Float%20%28single-precision%29))
  (bind _output_get (Variables|Default|SetCurXP (+ Recieved%20XP (Variables|Default|GetCurXP))))
  (while (>= _output_get (Variables|Default|GetReqXP))
    (Variables|Default|SetCurXP (- (Variables|Default|GetCurXP) (Variables|Default|GetReqXP)))))

(event Custom|Death
  (Utilities|FlowControl|DoOnce false
    (:Completed
      (Variables|Default|SetisDead true)
      (Physics|SetSimulatePhysics (Variables|Character|GetMesh) true)
      (Collision|SetCollisionEnabled (Variables|Collision|GetCapsuleComponent) "NoCollision")
      (Pawn|UnPossess (Pawn|GetController))
      (Utilities|FlowControl|Delay 2.0))))

(event EventBeginPlay
  (CallFunction|BeginHP)
  (CallFunction|SetDamage)
  (Variables|Default|SetSphereOffset (Transformation|GetWorldLocation (Variables|Default|GetSphere))))

(event EventTick
  (params (DeltaSeconds :type Float%20%28single-precision%29))
  (bind _outactors (Actor|GetAllActorsOfClass "/Game/Blueprints/Fighter.Fighter_C"))
  (for _array_element _outactors
    (if (not (Variables|/Game/Blueprints/Fighter.Fighter_C|GetisDead _array_element))
      (Variables|Default|SetLocation (Transformation|GetActorLocation _array_element))))
  (Transformation|SetWorldRotation (Variables|/Game/Blueprints/Equipment/TestSword.TestSword_C|GetSkeletalMesh (Variables|Default|GetSwordLeap)) (Math|Rotator|FindLookatRotation (Transformation|GetWorldLocation (Variables|/Game/Blueprints/Equipment/TestSword.TestSword_C|GetSkeletalMesh (Variables|Default|GetSwordLeap))) (Variables|Default|GetLocation)) false false))

(event EventRecieveDamage
  (params (HitInfo :type Hit%20Result%20Structure) (Damage :type Float%20%28single-precision%29) (Speed :type Float%20%28single-precision%29) (Weight :type Float%20%28single-precision%29))
  (bind (_bblockinghit _binitialoverlap _time _distance _location _impactpoint _normal _impactnormal _physmat _hitactor _hitcomponent _hitbonename) (Collision|BreakHitResult HitInfo))
  (bind (_x _y) (Math|Vector|BreakVector _location))
  (bind _returnvalue (Math|Conversions|RotationFromXVector _normal))
  (bind _output_get (Variables|Default|SetCurHP (- (Variables|Default|GetCurHP) Damage)))
  (if (>= _output_get 0.0)
    (Effects|SpawnEmitteratLocation "/Game/Effects/ParticleSystems/Gameplay/Player/P_body_bullet_impact.P_body_bullet_impact" _location _returnvalue "2.000000,2.000000,2.000000")
    (Class|GameplayStatics|SpawnDecalAttached "/Game/Materials/Mat_BloodDecal.Mat_BloodDecal" "64.000000,128.000000,128.000000" _hitcomponent _hitbonename _location _returnvalue "KeepWorldPosition" 0.0)
    (else
      (Effects|SpawnEmitteratLocation "/Game/Effects/ParticleSystems/Gameplay/Player/P_body_bullet_impact.P_body_bullet_impact" _location _returnvalue "4.000000,4.000000,4.000000")
      (Rendering|Decal|SpawnDecalatLocation "/Game/Materials/Mat_BloodDecal.Mat_BloodDecal" "128.000000,256.000000,256.000000" (Math|Vector|MakeVector _x _y 7e+02) "-90.000000,0.000000,0.000000" 0.0)
      (Class|SkeletalMeshComponent|BreakConstraint (Variables|Character|GetMesh) (* _normal -1e+03) _location _hitbonename)
      (CallFunction|Death))))

(event EventLeapRightHandMoved
  (params (hand :type Leap%20Hand%20Object%20Reference))
  (Transformation|SetWorldLocationAndRotation (Variables|Default|GetSphere) (- (+ (Variables|/Script/LeapMotion.LeapHand|GetWristPosition hand) (Transformation|GetActorLocation)) "0, 0,30.000000") (Variables|/Script/LeapMotion.LeapHand|GetPalmOrientation hand) false false))

(event Input|AxisEvents|InputAxisMoveForward
  (params (AxisValue :type Float%20%28single-precision%29))
  (Class|PawnMovementComponent|AddInputVector (Variables|Character|GetCharacterMovement) (* (Transformation|GetActorForwardVector (Game|GetPlayerCharacter 0)) AxisValue) false))

(event Input|AxisEvents|InputAxisMoveRight
  (params (AxisValue :type Float%20%28single-precision%29))
  (Class|PawnMovementComponent|AddInputVector (Variables|Character|GetCharacterMovement) (* (Transformation|GetActorRightVector (Game|GetPlayerCharacter 0)) AxisValue) false))

(fn ConstructionScript
  (bind _astest_sword (Utilities|Casting|CastToTestSword (Components|GetOwner (Components|GetChildComponent (Variables|Default|GetTestSword) 0))))
  (bind _output_get (Variables|Default|SetSwordLeap _astest_sword))
  (Transformation|AttachComponentToComponent (Variables|/Game/Blueprints/Equipment/TestSword.TestSword_C|GetSkeletalMesh _output_get) (Variables|Character|GetMesh) "SwordSocket2" "SnapToTarget" "KeepWorld" "KeepRelative" true))

(fn BeginHP
  (bind _output_get (Variables|Default|SetMaxHP (Math|Conversions|ToFloat(Integer) (+ (* (.Vitality (Utilities|Struct|BreakStruct_Fighter (Variables|Default|GetFighterInfo))) 10) 100))))
  (Variables|Default|SetCurHP _output_get))

(fn SetDamage
  (bind _fighterinfo (Variables|Default|GetFighterInfo))
  (bind (_id _name _level _strength _vitality _trainingpoints _curxp _reqxp _equippedsword) (Utilities|Struct|BreakStruct_Fighter _fighterinfo))
  (Variables|Default|SetDamage (+ (Math|Conversions|ToFloat(Integer) (* _strength 5)) (.Damage (Utilities|Struct|BreakStruct_Sword _equippedsword)))))