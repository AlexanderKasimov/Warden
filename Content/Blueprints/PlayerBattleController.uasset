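; Player controller for arena battles that turns input into movement, look and attacks for the player's fighter.
; A PossessPlayer event possesses the fighter held by the arena game mode and sets game-only input.
; Movement follows the pawn's forward and right vectors, while Attack calls the fighter's Attack2.
; With Leap Motion enabled, backward input disables orient-rotation-to-movement, and non-negative forward or any strafe axis update re-enables it.
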(event Custom|PossessPlayer
  (Pawn|Possess (Variables|/Game/Blueprints/ArenaGameMod_withPlayer.ArenaGameMod_withPlayer_C|GetPlayerFighter (Variables|Default|GetAGM_P)))
  (bind _asfighter_player (Utilities|Casting|CastToFighter_Player (Pawn|GetControlledPawn)))
  (Variables|Default|SetControlledPlayer _asfighter_player)
  (Input|SetInputModeGameOnly self))

(event EventBeginPlay
  (bind _asarena_game_mod_with_player (Utilities|Casting|CastToArenaGameMod_withPlayer (Game|GetGameMode)))
  (Variables|Default|SetAGM_P _asarena_game_mod_with_player))

(event EventTick
  (params (DeltaSeconds :type Float%20%28single-precision%29)))

(event Input|ActionEvents|InputActionAttack
  (params (Key :type Key%20Structure))
  (:Pressed
    (Default|Attack2 (Variables|Default|GetControlledPlayer))))

(event Input|AxisEvents|InputAxisMoveForward
  (params (AxisValue :type Float%20%28single-precision%29))
  (bind _controlledplayer (Variables|Default|GetControlledPlayer))
  (bind _charactermovement (Variables|/Script/Engine.Character|GetCharacterMovement _controlledplayer))
  (if (Variables|/Game/Blueprints/ArenaGameInstance.ArenaGameInstance_C|GetUseLeapMotion? (Variables|/Game/Blueprints/ArenaGameMod.ArenaGameMod_C|GetAGI (Variables|Default|GetAGM_P)))
    (if (< AxisValue 0.0)
      (Variables|/Script/Engine.CharacterMovementComponent|SetbOrientRotationToMovement _charactermovement false)
      (else
        (Variables|/Script/Engine.CharacterMovementComponent|SetbOrientRotationToMovement _charactermovement true))))
  (Pawn|Input|AddMovementInput _controlledplayer (Transformation|GetActorForwardVector _controlledplayer) AxisValue false))

(event Input|AxisEvents|InputAxisLookUp
  (params (AxisValue :type Float%20%28single-precision%29))
  (Class|PlayerController|AddPitchInput AxisValue))

(event Input|AxisEvents|InputAxisLookRight
  (params (AxisValue :type Float%20%28single-precision%29))
  (Class|PlayerController|AddYawInput AxisValue))

(event Input|AxisEvents|InputAxisMoveRight
  (params (AxisValue :type Float%20%28single-precision%29))
  (bind _controlledplayer (Variables|Default|GetControlledPlayer))
  (if (Variables|/Game/Blueprints/ArenaGameInstance.ArenaGameInstance_C|GetUseLeapMotion? (Variables|/Game/Blueprints/ArenaGameMod.ArenaGameMod_C|GetAGI (Variables|Default|GetAGM_P)))
    (Variables|/Script/Engine.CharacterMovementComponent|SetbOrientRotationToMovement (Variables|/Script/Engine.Character|GetCharacterMovement (Variables|Default|GetControlledPlayer)) true))
  (Pawn|Input|AddMovementInput _controlledplayer (Transformation|GetActorRightVector _controlledplayer) AxisValue false))

(fn ConstructionScript)