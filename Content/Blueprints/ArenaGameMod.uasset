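; Arena game mode that spawns the player and enemy fighter teams for a battle.
; Spawn points register through AddSpawner into per-team lists.
; On BeginPlay it initializes the player controller, waits briefly, then spawns a Fighter for each entry in the controller's two fighter lists.
; Spawn points are matched by index and supply transform and team, then all Fighters are sorted into team arrays.
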(event Custom|AddSpawner
  (params (Team :type Enum_TeamsList%20Enum :default "NewEnumerator0") (SpawnPoint :type Spawn%20Point%20Object%20Reference))
  (switch Utilities|FlowControl|Switch|SwitchonEnum_TeamsList Team
    (:NewEnumerator0
      (Development|PrintString "None team spawner"))
    (:NewEnumerator1
      (Utilities|Array|Add (Variables|Default|GetPlayerTeamSpawners) SpawnPoint))
    (:NewEnumerator2
      (Utilities|Array|Add (Variables|Default|GetEnemyTeamSpawners) SpawnPoint))))

(event Custom|SpawnTeams
  (Utilities|SpawnTeamfromList (Variables|/Game/Blueprints/PlayerController.PlayerController_C|GetFightersInBattleList (Variables|Default|GetPlayerController)) (Variables|Default|GetPlayerTeamSpawners)
    (:Out
      (Utilities|SpawnTeamfromList (Variables|/Game/Blueprints/PlayerController.PlayerController_C|GetEnemyFighterList (Variables|Default|GetPlayerController)) (Variables|Default|GetEnemyTeamSpawners)
        (:Out
          (bind _outactors (Actor|GetAllActorsOfClass "/Game/Blueprints/Fighter.Fighter_C"))
          (for _array_element _outactors
            (switch Utilities|FlowControl|Switch|SwitchonEnum_TeamsList (Variables|/Game/Blueprints/Fighter.Fighter_C|GetTeam _array_element)
              (:NewEnumerator1
                (Utilities|Array|Add (Variables|Default|GetPlayerTeamArray) _array_element))
              (:NewEnumerator2
                (Utilities|Array|Add (Variables|Default|GetEnemyTeamArray) _array_element)))))))))

(event EventBeginPlay
  (bind _asplayer_controller (Utilities|Casting|CastToPlayerController (Game|GetPlayerController 0)))
  (bind _output_get (Variables|Default|SetPlayerController _asplayer_controller))
  (Default|ArenaGameModInit _output_get)
  (Utilities|FlowControl|Delay 1.0)
  (CallFunction|SpawnTeams))

(event EventTick
  (params (DeltaSeconds :type Float%20%28single-precision%29)))

(fn ConstructionScript)