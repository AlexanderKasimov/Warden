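; Team-based sword fighter that takes HP and damage from FighterInfo in arena mode; elsewhere it loops its attack on a timer.
; Chained timelines lerp a right-hand transform through the swing while sphere traces damage each enemy once and push physics props.
; Hits spawn blood effects; death breaks a bone constraint, ragdolls the mesh and asks ArenaGameMod to check the win condition.
; Also handles XP level-ups and a player-facing info label.
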(event Custom|ExpRecieved
  (params (Recieved%20XP :type Float%20%28single-precision%29))
  (bind _output_get (Variables|Default|SetCurHP (+ Recieved%20XP (Variables|Default|GetCurXP))))
  (while (>= _output_get (Variables|Default|GetReqXP))
    (Variables|Default|SetCurHP (- (Variables|Default|GetCurXP) (Variables|Default|GetReqXP)))
    (Variables|Default|SetReqXP (* (Variables|Default|GetReqXP) 1.2))
    (Math|Integer|IncrementInt (Variables|Default|GetLVL))))

(event Custom|Death
  (Utilities|FlowControl|DoOnce false
    (:Completed
      (Variables|Default|SetisDead true)
      (Physics|SetSimulatePhysics (Variables|Character|GetMesh) true)
      (Collision|SetCollisionEnabled (Variables|Collision|GetCapsuleComponent) "NoCollision")
      (Pawn|UnPossess (Pawn|GetController))
      (Components|DestroyComponent (Variables|Default|GetInfo))
      (Utilities|FlowControl|Delay 2.0)
      (bind _asarena_game_mod (Utilities|Casting|CastToArenaGameMod (Game|GetGameMode)))
      (Default|CheckWinCondition _asarena_game_mod (Variables|Default|GetTeam)))))

(event Custom|PlaceHands
  (bind _newtrack_0 (Timeline|Timeline_PlaceHands Play)
    (:Update
      (Variables|Default|SetRightHandTransform (Math|Transform|Lerp(Transform) (Transformation|GetWorldTransform (Variables|Default|GetStartPlaceHands)) (Transformation|GetWorldTransform (Variables|Default|GetFinishPlaceHands)) _newtrack_0)))))

(event Custom|Attack_1
  (bind _target (Variables|Default|GetTarget))
  (bind _mesh (Variables|Character|GetMesh))
  (bind _returnvalue (Transformation|GetActorLocation _target))
  (bind _returnvalue_2 (Transformation|GetSocketLocation _mesh "SwordSocket"))
  (bind _returnvalue_3 (Math|Rotator|FindLookatRotation _returnvalue_2 _returnvalue))
  (Utilities|IsValid (Variables|Default|GetTarget)
    (:Is%20Valid
      (Transformation|SetWorldRotation (Variables|Default|GetAttack1_Vector) _returnvalue_3 false false)
      (Transformation|SetWorldLocationAndRotation (Variables|Default|GetEndAttack_1) _returnvalue _returnvalue_3 false false))
    (:Is%20Not%20Valid
      _))
  (Utilities|Array|Clear (Variables|Default|GetHittedEnemies))
  (bind _newtrack_0 (Timeline|Timeline_StartAttack_1 PlayFromStart)
    (:Update
      (Variables|Default|SetRightHandTransform (Math|Transform|Lerp(Transform) (Transformation|GetWorldTransform (Variables|Default|GetFinishPlaceHands)) (Transformation|GetWorldTransform (Variables|Default|GetStartAttack_1)) _newtrack_0)))
    (:Finished
      (bind _newtrack_1 (Timeline|Timeline_Attack_1 PlayFromStart)
        (:Update
          (Variables|Default|SetRightHandTransform (Math|Transform|Lerp(Transform) (Transformation|GetWorldTransform (Variables|Default|GetStartAttack_1)) (Transformation|GetWorldTransform (Variables|Default|GetEndAttack_1)) _newtrack_1))
          (Utilities|Attack1DamageDeal (Math|Rotator|Lerp(Rotator) "0.000000, 0, 0" (Transformation|GetWorldRotation (Variables|Default|GetAttack1_Vector)) _newtrack_1)))
        (:Finished
          (bind _newtrack_2 (Timeline|Timeline_Attack_1_Comeback PlayFromStart)
            (:Update
              (Variables|Default|SetRightHandTransform (Math|Transform|Lerp(Transform) (Transformation|GetWorldTransform (Variables|Default|GetEndAttack_1)) (Transformation|GetWorldTransform (Variables|Default|GetFinishPlaceHands)) _newtrack_2)))))))))

(event EventBeginPlay
  (bind _fighterinfo (Variables|Default|GetFighterInfo))
  (bind (_name _level) (Utilities|Struct|BreakStruct_Fighter _fighterinfo))
  (if (== (Utilities|GetClass (Game|GetGameMode)) "/Game/Blueprints/ArenaGameMod.ArenaGameMod_C")
    (CallFunction|BeginHP)
    (CallFunction|SetDamage)
    (Pawn|SpawnDefaultController)
    (CallFunction|PlaceHands)
    (Rendering|Components|TextRender|SetText (Variables|Default|GetInfo) (Utilities|Text|FormatText "{Name} 
LVL:{LVL} 
{Team}" _name _level (Utilities|Text|ToText(String) (Utilities|String|EnumtoString (Variables|Default|GetTeam)))))
    (Components|Timeline|SetPlayRate (Variables|Default|GetTimeline_StartAttack_1) 2.0)
    (Components|Timeline|SetPlayRate (Variables|Default|GetTimeline_Attack_1) 5.0)
    (Components|Timeline|SetPlayRate (Variables|Default|GetTimeline_Attack_1_Comeback) 2.0)
    (else
      (Rendering|SetVisibility (Variables|Default|GetInfo) false false)
      (CallFunction|PlaceHands)
      (Components|Timeline|SetPlayRate (Variables|Default|GetTimeline_StartAttack_1) 2.0)
      (Components|Timeline|SetPlayRate (Variables|Default|GetTimeline_Attack_1) 5.0)
      (Components|Timeline|SetPlayRate (Variables|Default|GetTimeline_Attack_1_Comeback) 2.0)
      (Utilities|Time|SetTimerbyEvent (delegate Custom|Attack_1) 3.0 true))))

(event EventTick
  (params (DeltaSeconds :type Float%20%28single-precision%29))
  (bind _info (Variables|Default|GetInfo))
  (Utilities|IsValid (Variables|Default|GetInfo)
    (:Is%20Valid
      (Transformation|SetWorldRotation _info (Math|Rotator|FindLookatRotation (Transformation|GetWorldLocation _info) (Transformation|GetActorLocation (Game|Player|GetPlayerPawn 0))) false false))))

(event EventRecieveDamage
  (params (HitInfo :type Hit%20Result%20Structure) (Damage :type Float%20%28single-precision%29))
  (bind (_bblockinghit _binitialoverlap _time _distance _location _impactpoint _normal _impactnormal _physmat _hitactor _hitcomponent _hitbonename) (Collision|BreakHitResult HitInfo))
  (bind (_x _y) (Math|Vector|BreakVector _location))
  (bind _returnvalue (Math|Conversions|RotationFromXVector _normal))
  (bind _output_get (Variables|Default|SetCurHP (- (Variables|Default|GetCurHP) Damage)))
  (if (>= _output_get 0.0)
    (Effects|SpawnEmitteratLocation "/Game/Effects/ParticleSystems/Gameplay/Player/P_body_bullet_impact.P_body_bullet_impact" _location _returnvalue "2.000000,2.000000,2.000000")
    (Class|GameplayStatics|SpawnDecalAttached "/Game/Materials/Mat_BloodDecal.Mat_BloodDecal" "64.000000,128.000000,128.000000" _hitcomponent _hitbonename _location _returnvalue "KeepWorldPosition" 0.0)
    (else
      (Effects|SpawnEmitteratLocation "/Game/Effects/ParticleSystems/Gameplay/Player/P_body_bullet_impact.P_body_bullet_impact" _location _returnvalue "4.000000,4.000000,4.000000")
      (Rendering|Decal|SpawnDecalatLocation "/Game/Materials/Mat_BloodDecal.Mat_BloodDecal" "128.000000,256.000000,256.000000" (Math|Vector|MakeVector _x _y 7e+02) "-90.000000,0.000000,0.000000" 0.0)
      (Class|SkeletalMeshComponent|BreakConstraint (Variables|Character|GetMesh) (* _normal -1e+03) _location _hitbonename)
      (CallFunction|Death))))

(fn ConstructionScript
  (bind _mesh (Variables|Character|GetMesh))
  (bind _returnvalue (AddComponent|AddSkeletalMeshComponent false (Transformation|GetSocketTransform _mesh "SwordSocket" "RTS_World")))
  (bind _output_get (Variables|Default|SetSword _returnvalue))
  (Transformation|AttachComponentToComponent _output_get _mesh "SwordSocket" "SnapToTarget" "SnapToTarget" "KeepRelative" true))

(fn BeginHP
  (bind _output_get (Variables|Default|SetMaxHP (Math|Conversions|ToFloat(Integer) (+ (* (.Vitality (Utilities|Struct|BreakStruct_Fighter (Variables|Default|GetFighterInfo))) 5) 100))))
  (Variables|Default|SetCurHP _output_get))

(fn SetDamage
  (bind _fighterinfo (Variables|Default|GetFighterInfo))
  (bind (_name _level _strength _vitality _trainingpoints _curxp _reqxp _equippedsword) (Utilities|Struct|BreakStruct_Fighter _fighterinfo))
  (Variables|Default|SetDamage (+ (Math|Conversions|ToFloat(Integer) (* _strength 5)) (.Damage (Utilities|Struct|BreakStruct_Sword _equippedsword)))))