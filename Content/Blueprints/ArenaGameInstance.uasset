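; Game instance for an arena game that holds the player, in-battle, enemy, shop and graveyard fighter lists plus player gold.
; SwapFighter and AddFighterToList resolve lists by type through SetOperandList, edit them, then write them back with SetSwappedList.
; UpdateIndexesInList re-stamps each fighter's stored array index after edits.
; SaveData and LoadData persist gold and all lists except the shop's through a SaveGame slot.
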(event Custom|SwapFighter
  (params (FighterIndex :type Integer) (FromList :type Enum_FighterListTypes%20Enum :default "NewEnumerator0") (ToList :type Enum_FighterListTypes%20Enum :default "NewEnumerator0"))
  (Variables|Default|SetFighterIndex FighterIndex)
  (Variables|Default|SetFromListType FromList)
  (Variables|Default|SetToListType ToList)
  (Variables|Default|SetFromList (CallFunction|SetOperandList (Variables|Default|GetFromListType)))
  (Variables|Default|SetToList (CallFunction|SetOperandList (Variables|Default|GetToListType)))
  (Utilities|Array|Add (Variables|Default|GetToList) (Utilities|Array|Get(acopy) (Variables|Default|GetFromList) (Variables|Default|GetFighterIndex)))
  (Utilities|Array|RemoveIndex (Variables|Default|GetFromList) (Variables|Default|GetFighterIndex))
  (Utilities|UpdateIndexesinList (Variables|Default|GetFromList)
    (:Out
      (Utilities|UpdateIndexesinList (Variables|Default|GetToList)
        (:Out
          (Utilities|SetSwappedList (Variables|Default|GetFromListType) (Variables|Default|GetFromList)
            (:Out
              (Utilities|SetSwappedList (Variables|Default|GetToListType) (Variables|Default|GetToList)))))))))

(event Custom|AddFighterToList
  (params (FighterInfo :type Struct%20Fighter%20Structure) (ListType :type Enum_FighterListTypes%20Enum :default "NewEnumerator0"))
  (Variables|Default|SetFighterInfo FighterInfo)
  (Variables|Default|SetToListType ListType)
  (bind _output_get (Variables|Default|SetToList (CallFunction|SetOperandList (Variables|Default|GetToListType))))
  (Utilities|Array|Add _output_get (Variables|Default|GetFighterInfo))
  (Utilities|UpdateIndexesinList (Variables|Default|GetToList)
    (:Out
      (Utilities|SetSwappedList (Variables|Default|GetToListType) (Variables|Default|GetToList)))))

(event Custom|LoadData
  (bind _returnvalue (SaveGame|DoesSaveGameExist (Variables|Default|GetSaveSlotName)))
  (bind _output_get (Variables|Default|SetSaveGameExist? _returnvalue))
  (if _output_get
    (bind _returnvalue_2 (SaveGame|LoadGamefromSlot (Variables|Default|GetSaveSlotName)))
    (bind _assave_game (Utilities|Casting|CastToSaveGame _returnvalue_2))
    (bind _output_get_2 (Variables|Default|SetSaveGame _assave_game))
    (Variables|Default|SetGeneralFighterList (Variables|/Game/Blueprints/SaveGame.SaveGame_C|GetPlayerFighterList _output_get_2))
    (Variables|Default|SetInBattleFighterList (Variables|/Game/Blueprints/SaveGame.SaveGame_C|GetFightersInBattleList (Variables|Default|GetSaveGame)))
    (Variables|Default|SetEnemyFighterList (Variables|/Game/Blueprints/SaveGame.SaveGame_C|GetEnemyFighterList (Variables|Default|GetSaveGame)))
    (Variables|Default|SetGraveyardList (Variables|/Game/Blueprints/SaveGame.SaveGame_C|GetGraveyardList (Variables|Default|GetSaveGame)))
    (Variables|Default|SetPlayerGold (Variables|/Game/Blueprints/SaveGame.SaveGame_C|GetPlayerGold (Variables|Default|GetSaveGame)))))

(event Custom|UpdateIndexesForShop
  (params (List :type Array%20of%20Struct%20Fighter%20Structures))
  (bind _outlist (Utilities|UpdateIndexesinList List)
    (:Out
      (Variables|Default|SetShopFighterList _outlist))))

(event Custom|UpdateIndexesForEnemyList
  (params (List :type Array%20of%20Struct%20Fighter%20Structures))
  (bind _outlist (Utilities|UpdateIndexesinList List)
    (:Out
      (Variables|Default|SetEnemyFighterList _outlist))))

(event Custom|SaveData
  (bind _returnvalue (SaveGame|CreateSaveGameObject "/Game/Blueprints/SaveGame.SaveGame_C"))
  (Variables|Default|SetSaveGame _returnvalue)
  (Variables|/Game/Blueprints/SaveGame.SaveGame_C|SetEnemyFighterList (Variables|Default|GetSaveGame) (Variables|Default|GetEnemyFighterList))
  (Variables|/Game/Blueprints/SaveGame.SaveGame_C|SetPlayerFighterList (Variables|Default|GetSaveGame) (Variables|Default|GetGeneralFighterList))
  (Variables|/Game/Blueprints/SaveGame.SaveGame_C|SetFightersInBattleList (Variables|Default|GetSaveGame) (Variables|Default|GetInBattleFighterList))
  (Variables|/Game/Blueprints/SaveGame.SaveGame_C|SetGraveyardList (Variables|Default|GetSaveGame) (Variables|Default|GetGraveyardList))
  (Variables|/Game/Blueprints/SaveGame.SaveGame_C|SetPlayerGold (Variables|Default|GetSaveGame) (Variables|Default|GetPlayerGold))
  (bind _returnvalue_2 (SaveGame|SaveGametoSlot (Variables|Default|GetSaveGame) (Variables|Default|GetSaveSlotName)))
  (if _returnvalue_2
    (Development|PrintString "Game saved" true true "(R=0.000000,G=1.000000,B=0.000000,A=1.000000)")
    (else
      (Development|PrintString "Save Failed!" true true "(R=1.000000,G=0.000000,B=0.000000,A=1.000000)"))))

(event Custom|ArrayInc
  (params (ArrayIN :type Array%20of%20Integers))
  (for (_array_element _array_index) ArrayIN
    (Utilities|Array|SetArrayElem ArrayIN _array_index (+ _array_element 1)))
  (Variables|Default|SetArray ArrayIN))

(fn SetOperandList
  (params (ListType :type Enum_FighterListTypes%20Enum :default "NewEnumerator0"))
  (switch Utilities|FlowControl|Switch|SwitchonEnum_FighterListTypes ListType
    (:NewEnumerator1
      (LocalVariables|SetLocalList (Variables|Default|GetGeneralFighterList)))
    (:NewEnumerator2
      (LocalVariables|SetLocalList (Variables|Default|GetEnemyFighterList)))
    (:NewEnumerator3
      (LocalVariables|SetLocalList (Variables|Default|GetShopFighterList)))
    (:NewEnumerator4
      (LocalVariables|SetLocalList (Variables|Default|GetInBattleFighterList))))
  (return (LocalVariables|GetLocalList)))