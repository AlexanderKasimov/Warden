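; Game mode for the main menu that starts a new arena game or continues a saved one.
; On BeginPlay it calls the player controller's MainMenuGameMode and caches the ArenaGameInstance.
; New game deletes the save slot, sets the NewGame flag and opens the prebattle level.
; Continue loads data through the game instance, then opens that level with the flag cleared, or prints an error when no save exists.
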(event Custom|StartNewGame
  (SaveGame|DeleteGameinSlot (Variables|/Game/Blueprints/ArenaGameInstance.ArenaGameInstance_C|GetSaveSlotName (Variables|Default|GetAGI)))
  (Variables|/Game/Blueprints/ArenaGameInstance.ArenaGameInstance_C|SetNewGame? (Variables|Default|GetAGI) true)
  (Game|OpenLevel(byName) "prebattle_v2"))

(event Custom|ContinueGame
  (Default|LoadData (Variables|Default|GetAGI))
  (if (Variables|/Game/Blueprints/ArenaGameInstance.ArenaGameInstance_C|GetSaveGameExist? (Variables|Default|GetAGI))
    (Variables|/Game/Blueprints/ArenaGameInstance.ArenaGameInstance_C|SetNewGame? (Variables|Default|GetAGI) false)
    (Game|OpenLevel(byName) "prebattle_v2")
    (else
      (Development|PrintString "No save game found!" true true "(R=1.000000,G=0.000000,B=0.000000,A=1.000000)"))))

(event EventBeginPlay
  (bind _asplayer_controller (Utilities|Casting|CastToPlayerController (Game|GetPlayerController 0)))
  (Default|MainMenuGameMode _asplayer_controller)
  (Variables|Default|SetAGI (.AsArena%20Game%20Instance (Utilities|Casting|CastToArenaGameInstance (Game|GetGameInstance)))))

(fn ConstructionScript)