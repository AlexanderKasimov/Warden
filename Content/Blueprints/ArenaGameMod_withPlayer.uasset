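; Arena game mode variant that sets up team battles which include a player-controlled fighter.
; On BeginPlay it initializes spawners, caches the ArenaGameInstance, spawns teams and builds team arrays, then has the PlayerBattleController possess the player.
; Its team spawn function places fighters at index-matched spawn points with their info and team, choosing Fighter_Player for the player type and storing it as PlayerFighter.
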(event EventBeginPlay
  (CallFunction|InitSpawners)
  (Variables|Default|SetAGI (.AsArena%20Game%20Instance (Utilities|Casting|CastToArenaGameInstance (Game|GetGameInstance))))
  (CallFunction|SpawnTeams)
  (CallFunction|InitTeamsArrays)
  (CallFunction|InitPlayerController))

(event EventInitPlayerController
  (bind _asplayer_battle_controller (Utilities|Casting|CastToPlayerBattleController (Game|GetPlayerController 0)))
  (bind _output_get (Variables|Default|SetPBC _asplayer_battle_controller))
  (Default|PossessPlayer _output_get))

(fn ConstructionScript
  (|CallParentFunction))

(fn SpawnTeamfromList(func)
  (params (FighterList :type Array%20of%20Struct%20Fighter%20Structures) (SpawnPointList :type Array%20of%20Spawn%20Point%20Object%20References))
  (for (_array_element _array_index) FighterList
    (LocalVariables|SetLocalFighter _array_element)
    (LocalVariables|SetLocalSpawnPoint (Utilities|Array|Get(acopy) SpawnPointList _array_index))
    (if (Utilities|Enum|Equal(Enum) (.FighterType (Utilities|Struct|BreakStruct_Fighter (LocalVariables|GetLocalFighter))) "NewEnumerator1")
      (bind _returnvalue (Game|SpawnActorfromClass "/Game/Blueprints/Fighter_Player.Fighter_Player_C" (Transformation|GetWorldTransform (Variables|/Game/Blueprints/SpawnPoint.SpawnPoint_C|GetSphere (LocalVariables|GetLocalSpawnPoint))) "Undefined" 0 (LocalVariables|GetLocalFighter) (Variables|/Game/Blueprints/SpawnPoint.SpawnPoint_C|GetTeam (LocalVariables|GetLocalSpawnPoint)) 0))
      (Variables|Default|SetPlayerFighter _returnvalue)
      (else
        (Game|SpawnActorfromClass "/Game/Blueprints/Fighter.Fighter_C" (Transformation|GetWorldTransform (Variables|/Game/Blueprints/SpawnPoint.SpawnPoint_C|GetSphere (LocalVariables|GetLocalSpawnPoint))) "Undefined" 0 (LocalVariables|GetLocalFighter) (Variables|/Game/Blueprints/SpawnPoint.SpawnPoint_C|GetTeam (LocalVariables|GetLocalSpawnPoint)) 0)))))