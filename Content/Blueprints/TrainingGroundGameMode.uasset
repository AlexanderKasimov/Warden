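; Game mode for the training ground, where the player buys fighters, picks a battle team and launches the arena level.
; Fighter lists and gold live in ArenaGameInstance; the mode moves fighters between lists, refreshes the TrainingGroundUI and saves before battle.
; Shop and enemy fighters are randomly generated from name and XP data tables, with levels scaled to the general list's average.
; A new game seeds a starter player fighter and gold.
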(event Custom|GenerateFightersShopList
  (bind _outgeneratedlist (CallFunction|GenerateFightersList (Variables|Default|GetGeneralFighterList) "NewEnumerator3"))
  (Default|SetList (Variables|Default|GetAGI) "NewEnumerator3" _outgeneratedlist))

(event Custom|BuyFighter
  (params (FighterInfo :type Struct%20Fighter%20Structure))
  (bind (_id _level) (Utilities|Struct|BreakStruct_Fighter FighterInfo))
  (if (>= (- (Variables|/Game/Blueprints/ArenaGameInstance.ArenaGameInstance_C|GetPlayerGold (Variables|Default|GetAGI)) (Math|Conversions|ToFloat(Integer) _level)) 0.0)
    (Default|SwapFighter (Variables|Default|GetAGI) _id "NewEnumerator3" "NewEnumerator1")
    (Variables|/Game/Blueprints/ArenaGameInstance.ArenaGameInstance_C|SetPlayerGold (Variables|Default|GetAGI) (- (Variables|/Game/Blueprints/ArenaGameInstance.ArenaGameInstance_C|GetPlayerGold (Variables|Default|GetAGI)) (Math|Conversions|ToFloat(Integer) _level)))
    (Default|UpdateFighterShopList (Variables|Default|GetTGUI))
    (Default|UpdatePlayerFighterList (Variables|Default|GetTGUI))
    (Development|PrintText (Utilities|Text|FormatText "{Result} ! {Cons} " (Utilities|Text|MakeLiteralText "Transaction Complete")) true true "(R=0.203919,G=1.000000,B=0.000000,A=1.000000)")
    (else
      (Development|PrintText (Utilities|Text|FormatText "{Result} ! {Cons} " (Utilities|Text|MakeLiteralText "Transaction Failed") (Utilities|Text|FormatText "{Result} {Value} {Type} " (Utilities|Text|MakeLiteralText "You need") _level (Utilities|Text|MakeLiteralText "gold"))) true true "(R=1.000000,G=0.007701,B=0.000000,A=1.000000)"))))

(event Custom|RemoveFighterFromBattleList
  (params (FighterInfo :type Struct%20Fighter%20Structure))
  (Default|SwapFighter (Variables|Default|GetAGI) (.ID (Utilities|Struct|BreakStruct_Fighter FighterInfo)) "NewEnumerator4" "NewEnumerator1")
  (Default|UpdatePlayerFighterList (Variables|Default|GetTGUI))
  (Default|UpdateFightersinBattleList (Variables|Default|GetTGUI)))

(event Custom|StartBattle
  (bind _agi (Variables|Default|GetAGI))
  (bind _inbattlefighterlist (Variables|/Game/Blueprints/ArenaGameInstance.ArenaGameInstance_C|GetInBattleFighterList _agi))
  (bind _returnvalue (Utilities|Array|Length _inbattlefighterlist))
  (if (> _returnvalue 0)
    (if (<= _returnvalue 5)
      (Default|SaveData (Variables|Default|GetAGI))
      (Game|OpenLevel(byName) "Arena_v2")
      (else
        (Development|PrintText "5 Fighters Max!!!" true true "(R=1.000000,G=0.008842,B=0.000000,A=1.000000)")))
    (else
      (Development|PrintText "You don't set any fighters!" true true "(R=1.000000,G=0.008842,B=0.000000,A=1.000000)"))))

(event Custom|FindBattle
  (bind _outgeneratedlist (CallFunction|GenerateFightersList (Variables|Default|GetGeneralFighterList) "NewEnumerator2"))
  (Default|SetList (Variables|Default|GetAGI) "NewEnumerator2" _outgeneratedlist))

(event Custom|AddFighterToBattleList
  (params (FighterInfo :type Struct%20Fighter%20Structure))
  (Default|SwapFighter (Variables|Default|GetAGI) (.ID (Utilities|Struct|BreakStruct_Fighter FighterInfo)) "NewEnumerator1" "NewEnumerator4")
  (Default|UpdatePlayerFighterList (Variables|Default|GetTGUI))
  (Default|UpdateFightersinBattleList (Variables|Default|GetTGUI)))

(event EventBeginPlay
  (bind _asplayer_controller (Utilities|Casting|CastToPlayerController (Game|GetPlayerController 0)))
  (bind _output_get (Variables|Default|SetPlayerController _asplayer_controller))
  (Default|TrainingGameModeInit _output_get)
  (Variables|Default|SetAGI (.AsArena%20Game%20Instance (Utilities|Casting|CastToArenaGameInstance (Game|GetGameInstance))))
  (Variables|Default|SetTGUI (Variables|/Game/Blueprints/PlayerController.PlayerController_C|GetTrainingGroundUI (Variables|Default|GetPlayerController)))
  (if (Variables|/Game/Blueprints/ArenaGameInstance.ArenaGameInstance_C|GetNewGame? (Variables|Default|GetAGI))
    (CallFunction|InitNewGame)
    (else
      (Default|UpdatePlayerFighterList (Variables|Default|GetTGUI)))))

(fn ConstructionScript)

(fn GenerateFightersList
  (params (GeneralFighterList :type Array%20of%20Struct%20Fighter%20Structures) (ListType :type Enum_FighterListTypes%20Enum :default "NewEnumerator0"))
  (LocalVariables|SetLocalGeneralFighterList GeneralFighterList)
  (switch Utilities|FlowControl|Switch|SwitchonEnum_FighterListTypes ListType
    (:NewEnumerator2
      (LocalVariables|SetNumberOfFighters (Math|Random|RandomIntegerinRange 1 5)))
    (:NewEnumerator3
      _))
  (for _array_element (LocalVariables|GetLocalGeneralFighterList)
    (LocalVariables|SetaverageLVL (+ (LocalVariables|GetaverageLVL) (.Level (Utilities|Struct|BreakStruct_Fighter _array_element)))))
  (LocalVariables|SetaverageLVL (/ (LocalVariables|GetaverageLVL) (Utilities|Array|Length (LocalVariables|GetLocalGeneralFighterList))))
  (LocalVariables|SetminLVL 1)
  (LocalVariables|SetmaxLVL (+ (LocalVariables|GetaverageLVL) (Math|Random|RandomIntegerinRange 1 2)))
  (for _index (range 0 (- (LocalVariables|GetNumberOfFighters) 1))
    (bind _outrownames (DataTable|GetDataTableRowNames "/Game/Blueprints/DataTables/Names.Names"))
    (bind _returnvalue (Utilities|GetDataTableRow "/Game/Blueprints/DataTables/Names.Names" (Utilities|Array|Get(acopy) _outrownames (Math|Random|RandomIntegerinRange 0 (- (Utilities|Array|Length _outrownames) 1))))
      (:then
        (LocalVariables|SetLVL (Math|Random|RandomIntegerinRange (LocalVariables|GetminLVL) (LocalVariables|GetmaxLVL)))
        (bind _returnvalue_2 (Utilities|GetDataTableRow "/Game/Blueprints/DataTables/ExpList.ExpList" (Utilities|String|StringToName (Utilities|String|ToString(Integer) (- (LocalVariables|GetLVL) 1))))
          (:then
            (Utilities|Array|Add (LocalVariables|GetLocalGeneratedList) (Utilities|Struct|MakeStruct_Fighter (Variables|/Game/Blueprints/ArenaGameInstance.ArenaGameInstance_C|GetIDCounter (Variables|Default|GetAGI)) (Utilities|Struct|BreakFigthersNames_Struct _returnvalue) (LocalVariables|GetLVL) (Math|Random|RandomIntegerinRange 1 (LocalVariables|GetLVL)) (- (LocalVariables|GetLVL) (Math|Random|RandomIntegerinRange 1 (LocalVariables|GetLVL))) 0 0.0 (Math|Conversions|ToFloat(Integer) (Math|Float|Round (Utilities|Struct|BreakLvlList_Struct _returnvalue_2))) (Utilities|Struct|MakeStruct_Sword "/Game/Meshes/SkeletalMeshes/Sword_Test_1/Sword_Test_1_SM.Sword_Test_1_SM" 2.0 2e+01) -1 "NewEnumerator2"))
            (Math|Integer|IncrementInt (Variables|/Game/Blueprints/ArenaGameInstance.ArenaGameInstance_C|GetIDCounter (Variables|Default|GetAGI))))))))
  (return (LocalVariables|GetLocalGeneratedList)))

(fn GeneratePlayerCharacter
  (params (Name :type Text) (Weapon :type Struct%20Sword%20Structure) (Level :type Integer))
  (LocalVariables|SetLocalName Name)
  (LocalVariables|SetLocalWeapon Weapon)
  (LocalVariables|SetLocalLevel Level)
  (bind _returnvalue (Utilities|GetDataTableRow "/Game/Blueprints/DataTables/ExpList.ExpList" (Utilities|String|StringToName (Utilities|String|ToString(Integer) (- (LocalVariables|GetLocalLevel) 1))))
    (:then
      (Math|Integer|IncrementInt (Variables|/Game/Blueprints/ArenaGameInstance.ArenaGameInstance_C|GetIDCounter (Variables|Default|GetAGI))
        (:%20%20
          (return (Utilities|Struct|MakeStruct_Fighter (Variables|/Game/Blueprints/ArenaGameInstance.ArenaGameInstance_C|GetIDCounter (Variables|Default|GetAGI)) (LocalVariables|GetLocalName) (LocalVariables|GetLocalLevel) 0 0 (LocalVariables|GetLocalLevel) 0.0 (Math|Conversions|ToFloat(Integer) (Math|Float|Round (Utilities|Struct|BreakLvlList_Struct _returnvalue))) (LocalVariables|GetLocalWeapon) -1 "NewEnumerator1")))))))

(fn InitNewGame
  (Default|AddFightertoList (Variables|Default|GetAGI) (CallFunction|GeneratePlayerCharacter "Player" (Utilities|Struct|MakeStruct_Sword "/Game/Meshes/SkeletalMeshes/Sword_Test_1/Sword_Test_1_SM.Sword_Test_1_SM" 2.0 2e+01) 3) "NewEnumerator1")
  (Default|UpdatePlayerFighterList (Variables|Default|GetTGUI))
  (Variables|/Game/Blueprints/ArenaGameInstance.ArenaGameInstance_C|SetPlayerGold (Variables|Default|GetAGI) (Variables|Default|GetPlayerGold))
  (Variables|/Game/Blueprints/ArenaGameInstance.ArenaGameInstance_C|SetNewGame? (Variables|Default|GetAGI) false))