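; Player controller for a fighter-team battle game, handling pawn input, main menu, training ground and arena setup, and persistent roster and gold.
; Moves fighters between roster and battle lists, re-indexing them, and generates random bandit enemies around the roster's average level.
; Arena setup derives gold and XP rewards from team danger difference and average level.
; Wins level survivors via a data table; losses discard the battle team; both save and reload pre-battle.
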(event Custom|TrainingGameModeInit
  (bind _fightersinbattlelist (Variables|Default|GetFightersInBattleList))
  (CallFunction|LoadData)
  (Variables|Default|SetbShowMouseCursor true)
  (bind _returnvalue (UserInterface|CreateWidget "/Game/UI/UI_TrainingGround.UI_TrainingGround_C"))
  (bind _output_get (Variables|Default|SetTrainingGroundUI _returnvalue))
  (UserInterface|Viewport|AddtoViewport _output_get 0)
  (Input|SetInputModeUIOnly self 0 "DoNotLock")
  (if (> (Utilities|Array|Length _fightersinbattlelist) 0)
    (for _array_element _fightersinbattlelist
      (CallFunction|AddFightertoList _array_element))
    (Utilities|UpdateIndexesinList (Variables|Default|GetPlayerFighterList)
      (:Out
        (Utilities|Array|Clear (Variables|Default|GetFightersInBattleList))
        (Default|UpdatePlayerFighterList (Variables|Default|GetTrainingGroundUI))))
    (else
      (Default|UpdatePlayerFighterList (Variables|Default|GetTrainingGroundUI)))))

(event Custom|ArenaGameModInit
  (CallFunction|LoadData)
  (Input|SetInputModeGameOnly self)
  (Variables|Default|SetbShowMouseCursor false)
  (Utilities|FlowControl|Delay 0.2)
  (CallFunction|UpdateBattleDanger)
  (CallFunction|CountAverageLVLinList)
  (bind _newreward (CallFunction|CalculateReward (Math|Conversions|ToFloat(Integer) (Variables|Default|GetavgLVL))))
  (bind _output_get (Variables|Default|SetFinalReward _newreward))
  (bind _newreward_2 (CallFunction|CalculateReward (Math|Conversions|ToFloat(Integer) (+ (Variables|Default|GetavgLVL) 300))))
  (bind _output_get_2 (Variables|Default|SetExpReward _newreward_2))
  (Development|PrintText (Utilities|Text|FormatText "BattleDanger:  {dgr} 
AVG lvl:  {avg} 
Reward Gold:  {grw} 
Reward XP:  {xrw}" (Variables|Default|GetbattleDanger) (Variables|Default|GetavgLVL) _output_get _output_get_2)))

(event Custom|CountAverageLVL%20in%20List
  (Variables|Default|SetavgLVL 0)
  (for _array_element (Variables|Default|GetFightersInBattleList)
    (Variables|Default|SetavgLVL (+ (Variables|Default|GetavgLVL) (.Level (Utilities|Struct|BreakStruct_Fighter _array_element)))))
  (Variables|Default|SetavgLVL (/ (Variables|Default|GetavgLVL) (Utilities|Array|Length (Variables|Default|GetFightersInBattleList)))))

(event Custom|FindBattle
  (bind _playerfighterlist (Variables|Default|GetPlayerFighterList))
  (Utilities|Array|Clear (Variables|Default|GetEnemyFighterList))
  (Variables|Default|SetaverageLVL 0)
  (for _array_element _playerfighterlist
    (Variables|Default|SetaverageLVL (+ (Variables|Default|GetaverageLVL) (.Level (Utilities|Struct|BreakStruct_Fighter _array_element)))))
  (Variables|Default|SetaverageLVL (/ (Variables|Default|GetaverageLVL) (Utilities|Array|Length _playerfighterlist)))
  (if (> (Variables|Default|GetaverageLVL) 2)
    (Variables|Default|SetminLVL (- (Variables|Default|GetaverageLVL) 1))
    (elif (== (Variables|Default|GetaverageLVL) 0)
      (Variables|Default|SetminLVL 1)
      (else
        (Variables|Default|SetminLVL (Variables|Default|GetaverageLVL)))))
  (Variables|Default|SetmaxLVL (+ (Variables|Default|GetaverageLVL) (Math|Random|RandomIntegerinRange 0 1)))
  (for _index (range 0 (- (Math|Random|RandomIntegerinRange 1 5) 1))
    (Variables|Default|SetLVL (Math|Random|RandomIntegerinRange (Variables|Default|GetminLVL) (Variables|Default|GetmaxLVL)))
    (Utilities|Array|Add (Variables|Default|GetEnemyFighterList) (Utilities|Struct|MakeStruct_Fighter (Utilities|Text|ToText(String) (Utilities|String|Append "Bandit_" (Utilities|String|ToString(Integer) (Math|Random|RandomIntegerinRange 0 199)))) (Variables|Default|GetLVL) (- (Variables|Default|GetLVL) (Math|Random|RandomIntegerinRange 1 (Variables|Default|GetLVL))) (Math|Random|RandomIntegerinRange 1 (Variables|Default|GetLVL)) 0 0.0 0.0 (Utilities|Struct|MakeStruct_Sword "/Game/Meshes/SkeletalMeshes/Sword_Test_1/Sword_Test_1_SM.Sword_Test_1_SM" 5e+02 2e+01) -1))))

(event Custom|Remove%20Fighter%20At%20Index%20From%20Battle%20List
  (params (Index :type Integer))
  (bind _traininggroundui (Variables|Default|GetTrainingGroundUI))
  (Utilities|Array|Add (Variables|Default|GetPlayerFighterList) (Utilities|Array|Get(acopy) (Variables|Default|GetFightersInBattleList) Index))
  (Utilities|RemovefromListatIndex (Variables|Default|GetFightersInBattleList) Index
    (:Out
      (Utilities|UpdateIndexesinList (Variables|Default|GetPlayerFighterList)
        (:Out
          (Utilities|UpdateIndexesinList (Variables|Default|GetFightersInBattleList)
            (:Out
              (Default|UpdatePlayerFighterList _traininggroundui)
              (Default|UpdateFightersinBattleList _traininggroundui))))))))

(event Custom|Win
  (params (PlayerTeamArray :type Array%20of%20Fighter%20Object%20References))
  (Utilities|Array|Clear (Variables|Default|GetEnemyFighterList))
  (for _array_element PlayerTeamArray
    (if (not (Variables|/Game/Blueprints/Fighter.Fighter_C|GetisDead _array_element))
      (Utilities|Array|SetArrayElem (Variables|Default|GetFightersInBattleList) (.IndexInPlayerArray (Utilities|Struct|BreakStruct_Fighter (Variables|/Game/Blueprints/Fighter.Fighter_C|GetFighterInfo _array_element))) (Variables|/Game/Blueprints/Fighter.Fighter_C|GetFighterInfo _array_element))))
  (for _array_element_2 PlayerTeamArray
    (if (Variables|/Game/Blueprints/Fighter.Fighter_C|GetisDead _array_element_2)
      (Utilities|RemovefromListatIndex (Variables|Default|GetFightersInBattleList) (.IndexInPlayerArray (Utilities|Struct|BreakStruct_Fighter (Variables|/Game/Blueprints/Fighter.Fighter_C|GetFighterInfo _array_element_2))))))
  (for _array_element_3 (Variables|Default|GetFightersInBattleList)
    (bind (_newcurxp _newreqxp _newlvl _newtrainingpoints) (CallFunction|AddXP (Variables|Default|GetExpReward) (.CurXP (Utilities|Struct|BreakStruct_Fighter _array_element_3)) (.ReqXP (Utilities|Struct|BreakStruct_Fighter _array_element_3)) (.Level (Utilities|Struct|BreakStruct_Fighter _array_element_3)) (.TrainingPoints (Utilities|Struct|BreakStruct_Fighter _array_element_3))))
    (Utilities|Array|Add (Variables|Default|GetPlayerFighterList) (Utilities|Struct|MakeStruct_Fighter (.Name (Utilities|Struct|BreakStruct_Fighter _array_element_3)) _newlvl (.Strength (Utilities|Struct|BreakStruct_Fighter _array_element_3)) (.Vitality (Utilities|Struct|BreakStruct_Fighter _array_element_3)) _newtrainingpoints (Math|Conversions|ToFloat(Integer) (Math|Float|Round _newcurxp)) (Math|Conversions|ToFloat(Integer) (Math|Float|Round _newreqxp)) (.EquippedSword (Utilities|Struct|BreakStruct_Fighter _array_element_3)) (.IndexInPlayerArray (Utilities|Struct|BreakStruct_Fighter _array_element_3)))))
  (Utilities|UpdateIndexesinList (Variables|Default|GetPlayerFighterList)
    (:Out
      (Utilities|Array|Clear (Variables|Default|GetFightersInBattleList))
      (Variables|Default|SetGold (+ (Variables|Default|GetGold) (Math|Conversions|ToFloat(Integer) (Math|Float|Round (Variables|Default|GetFinalReward)))))
      (CallFunction|SaveData)
      (Utilities|FlowControl|Delay 5.0)
      (Game|OpenLevel(byName) "prebattle_v2"))))

(event Custom|Save%20Data
  (bind _returnvalue (SaveGame|CreateSaveGameObject "/Game/Blueprints/SaveGame.SaveGame_C"))
  (bind _output_get (Variables|Default|SetSaveGame _returnvalue))
  (Variables|/Game/Blueprints/SaveGame.SaveGame_C|SetEnemyFighterList _output_get (Variables|Default|GetEnemyFighterList))
  (Variables|/Game/Blueprints/SaveGame.SaveGame_C|SetPlayerFighterList _output_get (Variables|Default|GetPlayerFighterList))
  (Variables|/Game/Blueprints/SaveGame.SaveGame_C|SetGold _output_get (Variables|Default|GetGold))
  (Variables|/Game/Blueprints/SaveGame.SaveGame_C|SetFightersInBattleList _output_get (Variables|Default|GetFightersInBattleList))
  (bind _returnvalue_2 (SaveGame|SaveGametoSlot (Variables|Default|GetSaveGame) (Variables|Default|GetPlayerControllerSaveSlot)))
  (if _returnvalue_2
    (Development|PrintString "Game saved" true true "(R=0.000000,G=1.000000,B=0.000000,A=1.000000)")
    (else
      (Development|PrintString "Save Failed!" true true "(R=1.000000,G=0.000000,B=0.000000,A=1.000000)"))))

(event Custom|UpdateBattleDanger
  (Variables|Default|SetplayerTeamDanger 0)
  (for _array_element (Variables|Default|GetFightersInBattleList)
    (Variables|Default|SetplayerTeamDanger (+ (Variables|Default|GetplayerTeamDanger) 25 (.Level (Utilities|Struct|BreakStruct_Fighter _array_element)))))
  (Variables|Default|SetenemyTeamDanger 0)
  (for _array_element_2 (Variables|Default|GetEnemyFighterList)
    (Variables|Default|SetenemyTeamDanger (+ (Variables|Default|GetenemyTeamDanger) 25 (.Level (Utilities|Struct|BreakStruct_Fighter _array_element_2)))))
  (Variables|Default|SetbattleDanger (- (Variables|Default|GetenemyTeamDanger) (Variables|Default|GetplayerTeamDanger))))

(event Custom|LoadData
  (bind _returnvalue (SaveGame|DoesSaveGameExist (Variables|Default|GetPlayerControllerSaveSlot)))
  (if _returnvalue
    (bind _returnvalue_2 (SaveGame|LoadGamefromSlot (Variables|Default|GetPlayerControllerSaveSlot)))
    (bind _assave_game (Utilities|Casting|CastToSaveGame _returnvalue_2))
    (bind _output_get (Variables|Default|SetSaveGame _assave_game))
    (Variables|Default|SetPlayerFighterList (Variables|/Game/Blueprints/SaveGame.SaveGame_C|GetPlayerFighterList _output_get))
    (Variables|Default|SetEnemyFighterList (Variables|/Game/Blueprints/SaveGame.SaveGame_C|GetEnemyFighterList (Variables|Default|GetSaveGame)))
    (Variables|Default|SetFightersInBattleList (Variables|/Game/Blueprints/SaveGame.SaveGame_C|GetFightersInBattleList (Variables|Default|GetSaveGame)))
    (Variables|Default|SetGold (Variables|/Game/Blueprints/SaveGame.SaveGame_C|GetGold (Variables|Default|GetSaveGame)))
    (else
      (Development|PrintString "No save game found!" true true "(R=1.000000,G=0.000000,B=0.000000,A=1.000000)")
      (Variables|Default|SetGold (Variables|Default|GetDefaultGold)))))

(event Custom|Lose
  (Utilities|Array|Clear (Variables|Default|GetEnemyFighterList))
  (Utilities|Array|Clear (Variables|Default|GetFightersInBattleList))
  (CallFunction|SaveData)
  (Utilities|FlowControl|Delay 5.0)
  (Game|OpenLevel(byName) "prebattle_v2"))

(event Custom|Add%20Fighter%20At%20Index%20to%20Battle%20list
  (params (Index :type Integer))
  (bind _traininggroundui (Variables|Default|GetTrainingGroundUI))
  (Utilities|Array|Add (Variables|Default|GetFightersInBattleList) (Utilities|Array|Get(acopy) (Variables|Default|GetPlayerFighterList) Index))
  (Utilities|RemovefromListatIndex (Variables|Default|GetPlayerFighterList) Index
    (:Out
      (Utilities|UpdateIndexesinList (Variables|Default|GetPlayerFighterList)
        (:Out
          (Utilities|UpdateIndexesinList (Variables|Default|GetFightersInBattleList)
            (:Out
              (Default|UpdatePlayerFighterList _traininggroundui)
              (Default|UpdateFightersinBattleList _traininggroundui))))))))

(event Custom|Add%20Fighter%20to%20List
  (params (FighterInfo :type Struct%20Fighter%20Structure))
  ;[1 1 1] Возможно лучше функция
  (Utilities|Array|Add (Variables|Default|GetPlayerFighterList) FighterInfo)
  (Utilities|UpdateIndexesinList (Variables|Default|GetPlayerFighterList)
    (:Out
      (Default|UpdatePlayerFighterList (Variables|Default|GetTrainingGroundUI)))))

(event Custom|MainMenuGameMode
  (Variables|Default|SetbShowMouseCursor true)
  (bind _returnvalue (UserInterface|CreateWidget "/Game/UI/UI_MainMenu.UI_MainMenu_C"))
  (UserInterface|Viewport|AddtoViewport _returnvalue 0)
  (Input|SetInputModeUIOnly self 0 "DoNotLock"))

(event EventBeginPlay
  (bind _returnvalue (Pawn|GetControlledPawn))
  (bind (_asplayer_pawn _bsuccess) (Utilities|Casting|CastToPlayerPawn _returnvalue))
  (if _bsuccess
    (Variables|Default|SetPlayerPawn _asplayer_pawn)))

(event EventTick
  (params (DeltaSeconds :type Float%20%28single-precision%29)))

(event Input|AxisEvents|InputAxisMoveRight
  (params (AxisValue :type Float%20%28single-precision%29))
  (Class|PawnMovementComponent|AddInputVector (Variables|/Game/Blueprints/PlayerPawn.PlayerPawn_C|GetFloatingPawnMovement (Variables|Default|GetPlayerPawn)) (* (Math|Vector|GetRightVector (Pawn|GetControlRotation self :!class /Script/Engine.Controller)) AxisValue) false))

(event Input|AxisEvents|InputAxisLookUp
  (params (AxisValue :type Float%20%28single-precision%29))
  (Class|PlayerController|AddPitchInput (* AxisValue -1.0)))

(event Input|AxisEvents|InputAxisLookRight
  (params (AxisValue :type Float%20%28single-precision%29))
  (Class|PlayerController|AddYawInput AxisValue))

(event Input|AxisEvents|InputAxisMoveForward
  (params (AxisValue :type Float%20%28single-precision%29))
  (Class|PawnMovementComponent|AddInputVector (Variables|/Game/Blueprints/PlayerPawn.PlayerPawn_C|GetFloatingPawnMovement (Variables|Default|GetPlayerPawn)) (* (Math|Vector|GetForwardVector (Pawn|GetControlRotation self :!class /Script/Engine.Controller)) AxisValue) false))

(fn ConstructionScript)

(fn AddXP
  (params (AddedXP :type Float%20%28single-precision%29) (CurXP_F :type Float%20%28single-precision%29) (ReqXP_F :type Float%20%28single-precision%29) (LVL_F :type Integer) (trainingPoints_F :type Integer))
  (LocalVariables|SettrainingPoints_L trainingPoints_F)
  (LocalVariables|SetCurXP CurXP_F)
  (LocalVariables|SetReqXP ReqXP_F)
  (LocalVariables|SetLVL_L LVL_F)
  (bind _output_get (LocalVariables|SetCurXP (+ AddedXP (LocalVariables|GetCurXP))))
  (while (>= _output_get (LocalVariables|GetReqXP))
    (LocalVariables|SetCurXP (- (LocalVariables|GetCurXP) (LocalVariables|GetReqXP)))
    (Math|Integer|IncrementInt (LocalVariables|GetLVL_L)
      (:%20%20
        (Math|Integer|IncrementInt (LocalVariables|GettrainingPoints_L)
          (:%20%20
            (bind _returnvalue (Utilities|GetDataTableRow "/Game/Blueprints/DataTables/ExpList.ExpList" (Utilities|String|StringToName (Utilities|String|ToString(Integer) (- (LocalVariables|GetLVL_L) 1))))
              (:then
                (LocalVariables|SetReqXP (Math|Conversions|ToFloat(Integer) (Math|Float|Round (.EXP (Utilities|Struct|BreakLvlList_Struct _returnvalue))))))
              (:RowNotFound
                (Development|PrintString "Max LVL Reached"))))))))
  (return (LocalVariables|GetCurXP) (LocalVariables|GetReqXP) (LocalVariables|GetLVL_L) (LocalVariables|GettrainingPoints_L)))

(fn CalculateReward
  (params (BaseAmount :type Float%20%28single-precision%29))
  (Development|PrintText (Utilities|Text|FormatText "BaseAmount:{Am}" BaseAmount))
  (Math|Integer|CompareInt (Variables|Default|GetbattleDanger)
    (:>
      (LocalVariables|SetReward (* BaseAmount (Math|Conversions|ToFloat(Integer) (+ (/ (Variables|Default|GetbattleDanger) 5) 1)) (Math|Conversions|ToFloat(Integer) (Utilities|Array|Length (Variables|Default|GetFightersInBattleList))))))
    (:==
      (LocalVariables|SetReward (* (Utilities|Array|Length (Variables|Default|GetFightersInBattleList)) BaseAmount)))
    (:<
      (if (< (Variables|Default|GetbattleDanger) -100)
        (LocalVariables|SetReward (* BaseAmount (Math|Conversions|ToFloat(Integer) (Utilities|Array|Length (Variables|Default|GetFightersInBattleList))) 0.01))
        (else
          (LocalVariables|SetReward (* BaseAmount (Math|Conversions|ToFloat(Integer) (+ (/ (Variables|Default|GetbattleDanger) 100) 1)) (Math|Conversions|ToFloat(Integer) (Utilities|Array|Length (Variables|Default|GetFightersInBattleList)))))))))
  (return (LocalVariables|GetReward)))